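; Clickable prop for the room decoration feature that lets the player swap its mesh from a W_MeshList widget.
; Hover toggles custom depth; clicking shows the list and fires OpenedHUD, and HideHUD hides it.
; BeginPlay positions the list per a placement setting, initializes it from PropSettings and binds to its prop-changed event.
; The chosen prop's DT_RoomProps row supplies rotation and an offset from the initial position.
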(event `ResetMesh`
  (bind _asw_mesh_list (cast `/Game/DavideZanfardino/BP/HUD/MeshList/W_MeshList` (`WidgetComponent.GetUserWidgetObject` (`self.MeshList`))))
  (`StaticMeshComponent.SetStaticMesh` (`self.StaticMesh`) (`/Game/DavideZanfardino/BP/HUD/MeshList/W_MeshList.FinalPropMesh` _asw_mesh_list))
  (bind _finalpropenum (`/Game/DavideZanfardino/BP/HUD/MeshList/W_MeshList.FinalPropEnum` _asw_mesh_list))
  (bind _returnvalue (`|GetDataTableRow` "/Game/LucaCasamenti/DecorateRoom/DataTables/DT_RoomProps.DT_RoomProps" (`KismetStringLibrary.Conv_StringToName` (`|GetEnumeratorNameAsString` _finalpropenum)))
    (:`then`
      (`SceneComponent.K2_SetWorldRotation` (`self.StaticMesh`) (`.Rotation_21_6890F66B42AEAD20CE7B36A6CAFE7E55` (break `/Game/LucaCasamenti/DecorateRoom/Structures/S_Prop` _returnvalue)) false false)
      (`SceneComponent.K2_SetWorldLocation` (`self.StaticMesh`) (+ (`self.InitialPosition`) (`.Location_18_16F5C8814F91DACE58B6E195219713F3` (break `/Game/LucaCasamenti/DecorateRoom/Structures/S_Prop` _returnvalue))) false false)
      (set `self.ActualPropType` _finalpropenum)
      (set `self.ActualIndex` (`/Game/DavideZanfardino/BP/HUD/MeshList/W_MeshList.PropsIndex` _asw_mesh_list)))
    (:`RowNotFound`
      (`KismetSystemLibrary.PrintString` "non trovata ptrop in tabella"))))

(event `self.ReceiveBeginPlay`
  (bind (_propsettings_category _propsettings_prop) (break `/Game/LucaCasamenti/DecorateRoom/Structures/S_Prop` (`self.PropSettings`)))
  (bind (_propsettings_category_2 _propsettings_prop_2) (break `/Game/LucaCasamenti/DecorateRoom/Structures/S_Prop` (`self.PropSettings`)))
  (bind (_propsettings_category_3 _propsettings_prop_3) (break `/Game/LucaCasamenti/DecorateRoom/Structures/S_Prop` (`self.PropSettings`)))
  (bind (_propsettings_category_4 _propsettings_prop_4 _propsettings_mesh) (break `/Game/LucaCasamenti/DecorateRoom/Structures/S_Prop` (`self.PropSettings`)))
  (set `self.PropsListWidgetInitialPosition` (`SceneComponent.K2_GetComponentLocation` (`self.MeshList`)))
  (switch `/Game/LucaCasamenti/DecorateRoom/Enums/E_PropsListWidgetPosition` (`self.PropsListWidgetPosition`)
    (:`NewEnumerator0`
      (set `self.PropsListWidgetNewPosition` (+ (`self.PropsListWidgetInitialPosition`) (0.0 0.0 300.0))))
    (:`NewEnumerator1`
      (set `self.PropsListWidgetNewPosition` (`self.PropsListWidgetInitialPosition`)))
    (:`NewEnumerator2`
      (set `self.PropsListWidgetNewPosition` (+ (`self.PropsListWidgetInitialPosition`) (500.0 0.0 0.0))))
    (:`NewEnumerator3`
      (set `self.PropsListWidgetNewPosition` (+ (`self.PropsListWidgetInitialPosition`) (-100.0 0.0 0.0)))))
  (`SceneComponent.K2_SetWorldLocation` (`self.MeshList`) (`self.PropsListWidgetNewPosition`) false false)
  (set `self.InitialPosition` (`SceneComponent.K2_GetComponentLocation` (`self.StaticMesh`)))
  (bind _asw_mesh_list (cast `/Game/DavideZanfardino/BP/HUD/MeshList/W_MeshList` (`WidgetComponent.GetUserWidgetObject` (`self.MeshList`))))
  (`/Game/DavideZanfardino/BP/HUD/MeshList/W_MeshList.init` _asw_mesh_list _propsettings_prop_4 _propsettings_mesh _propsettings_category_4 (`self.ActualIndex`))
  (add `/Game/DavideZanfardino/BP/HUD/MeshList/W_MeshList.PropChanged` _asw_mesh_list (`|CreateDelegate` :!event `ResetMesh`))
  (set `self.ActualPropType` _propsettings_prop)
  (bind _returnvalue (`|GetDataTableRow` "/Game/LucaCasamenti/DecorateRoom/DataTables/DT_RoomProps.DT_RoomProps" (`KismetStringLibrary.Conv_StringToName` (`|GetEnumeratorNameAsString` _propsettings_prop_2)))
    (:`then`
      (`SceneComponent.K2_SetWorldRotation` (`self.StaticMesh`) (`.Rotation_21_6890F66B42AEAD20CE7B36A6CAFE7E55` (break `/Game/LucaCasamenti/DecorateRoom/Structures/S_Prop` _returnvalue)) false false)
      (`SceneComponent.K2_SetWorldLocation` (`self.StaticMesh`) (+ (`self.InitialPosition`) (`.Location_18_16F5C8814F91DACE58B6E195219713F3` (break `/Game/LucaCasamenti/DecorateRoom/Structures/S_Prop` _returnvalue))) false false)
      (set `self.ActualPropType` _propsettings_prop_3)
      (set `self.ActualIndex` (`self.ActualIndex`)))))

(event `self.StaticMesh.OnBeginCursorOver`
  (params (TouchedComponent :type "PrimitiveComponent Object Reference"))
  (`KismetSystemLibrary.PrintString` "Mouse in")
  (`GameplayStatics.PlaySound2D` "/Game/DavideZanfardino/Audio/FISH_AND_KISS_SOUND_2/STANZA/STANZA_MOUSE_ON/FISH_AND_KISS_STANZA_MOUSE_1.FISH_AND_KISS_STANZA_MOUSE_1" 0.6 1.0 0.0 null null)
  (`PrimitiveComponent.SetRenderCustomDepth` (`self.StaticMesh`) true))

(event `self.StaticMesh.OnEndCursorOver`
  (params (TouchedComponent :type "PrimitiveComponent Object Reference"))
  (`KismetSystemLibrary.PrintString` "Mouse out")
  (`PrimitiveComponent.SetRenderCustomDepth` (`self.StaticMesh`) false))

(event `self.StaticMesh.OnClicked`
  (params (TouchedComponent :type "PrimitiveComponent Object Reference") (ButtonPressed :type "Key Structure"))
  (`GameplayStatics.PlaySound2D` "/Game/DavideZanfardino/Audio/FISH_AND_KISS_SOUND_2/STANZA/STANZA_LISTA/FISH_AND_KISS_STANZA_LIST_1.FISH_AND_KISS_STANZA_LIST_1" 0.6 1.0 0.0 null null)
  (`self.OpenedHUD`)
  (`SceneComponent.SetVisibility` (`self.MeshList`) true false))

(event `HideHUD`
  (`SceneComponent.SetVisibility` (`self.MeshList`) false false))

(fn `UserConstructionScript`
  (bind (_propsettings_category _propsettings_prop _propsettings_mesh) (break `/Game/LucaCasamenti/DecorateRoom/Structures/S_Prop` (`self.PropSettings`)))
  (`StaticMeshComponent.SetStaticMesh` (`self.StaticMesh`) _propsettings_mesh))