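; GM_FishAndKiss is a game mode for a fishing game that tracks which fish is in focus.
; NextFish advances an index into FishesPool, which GetFishInFocus reads as a circular array using modulo.
; CatchFish is still a stub that only prints the name of the fish to catch.
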(event `NextFish`
  ;[1 1 1] For now, circular array
  (`/Engine/EditorBlueprintResources/StandardMacros.IncrementInt` (`self.FishesIndex`)))

(event `CatchFish`
  ;[1 1 1] Catch fish
  (bind _fish (`self.GetFishInFocus`))
  (`KismetSystemLibrary.PrintString` (`KismetStringLibrary.Concat_StrStr` "Devo catturare " (`.Name_9_F79A53BE47F503FFC775239A5E38C591` (break `/Game/LucaCasamenti/Fish/Structures/S_Fish` _fish)))))

(fn `GetFishInFocus`
  (returns (Fish :type "/Game/LucaCasamenti/Fish/Structures/S_Fish Structure"))
  ;[1 1 1] Circular array for now
  (return (`|GetArrayItem` (`self.FishesPool`) (mod (`self.FishesIndex`) (`KismetArrayLibrary.Array_Length` (`self.FishesPool`))))))

(fn `UserConstructionScript`)