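; BP_CaughtFish is the caught-fish actor that plays the catch presentation, rising out of the lake and flying to the camera.
; On BeginPlay, one timeline lifts it 500 units, then a second pulls it to just in front of the screen center, deprojected every update.
; Both lerp from the current location, so motion compounds each tick.
; When the second finishes, it calls CaughtScreen on GM_FishAndKiss.
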(event `self.ReceiveBeginPlay`
  (bind _returnvalue (`GameplayStatics.GetPlayerController` 0))
  (bind (_sizex _sizey) (`PlayerController.GetViewportSize` _returnvalue))
  (bind (_x _y _z) (`KismetMathLibrary.BreakVector3f` (`self.K2_GetActorLocation`)))
  (bind (_worldlocation _worlddirection) (`PlayerController.DeprojectScreenPositionToWorld` _returnvalue (`KismetMathLibrary.Conv_IntToDouble` (/ _sizex 2)) (`KismetMathLibrary.Conv_IntToDouble` (/ _sizey 2))))
  (set `self.FinalPosition` (`KismetMathLibrary.MakeVector` _x _y (+ _z 500.0)))
  ;[1 1 1] from underground to out of lake
  (bind (_direction _alpha) (`Timeline|Timeline`)
    (:`Update`
      (`self.K2_SetActorLocation` (`KismetMathLibrary.VLerp` (`self.K2_GetActorLocation`) (`self.FinalPosition`) _alpha)))
    (:`Finished`
      ;[1 1 1] From out of lake to front of camera
      (`KismetSystemLibrary.PrintString` "fine mi sono alzato")
      (bind (_direction_2 _newtrack_0) (`Timeline|Timeline_0`)
        (:`Update`
          (`self.K2_SetActorLocation` (`KismetMathLibrary.VLerp` (`self.K2_GetActorLocation`) (+ _worldlocation (* _worlddirection 100)) _newtrack_0)))
        (:`Finished`
          ;[1 1 1] Caught screen
          (bind _asgm_fish_and_kiss (cast `/Game/LucaCasamenti/GameplayFramework/GameModes/GM_FishAndKiss` (`GameplayStatics.GetGameMode`)))
          (`/Game/LucaCasamenti/GameplayFramework/GameModes/GM_FishAndKiss.CaughtScreen` _asgm_fish_and_kiss))))))

(fn `UserConstructionScript`)