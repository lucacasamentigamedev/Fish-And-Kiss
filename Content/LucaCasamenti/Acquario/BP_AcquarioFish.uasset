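; Aquarium fish actor that sets its static mesh and wanders at random around its spawn point.
; GetNewPosition picks random X and Z offsets from the location saved at BeginPlay, keeping Y fixed.
; A looping Move event waits briefly, nudges the RotatingMovement rate at random, then uses a timeline to lerp with sweep from the current location to the new point.
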(event `self.ReceiveBeginPlay`
  (set `self.CurrentPosition` (`self.K2_GetActorLocation`))
  (bind _newposition (`self.GetNewPosition`))
  (`self.K2_SetActorLocation` _newposition)
  ;[1 1 1] Qui setto la mesh ma se poi abbiamo la skeletal mesh allora possiamo provare a mettere quella e ad animarla
  (`StaticMeshComponent.SetStaticMesh` (`self.StaticMesh`) (`self.Mesh`))
  (`self.Move`))

(event `Move`
  (bind _returnvalue (`KismetMathLibrary.RandomFloatInRange` -5.0 5.0))
  (bind _rotatingmovement (`self.RotatingMovement`))
  (bind (_rotationrate_roll _rotationrate_pitch _rotationrate_yaw) (`KismetMathLibrary.BreakRotator` (`RotatingMovementComponent.RotationRate` _rotatingmovement)))
  (`KismetSystemLibrary.Delay` (`KismetMathLibrary.RandomFloatInRange` 0.1 1.0))
  (bind _newposition (`self.GetNewPosition`))
  ;[1 1 1] Randomize rotation
  (set `RotatingMovementComponent.RotationRate` (`KismetMathLibrary.MakeRotator` (+ _rotationrate_roll _returnvalue) (+ _rotationrate_pitch _returnvalue) (+ _rotationrate_yaw _returnvalue)) _rotatingmovement)
  ;[1 1 1] Move and restart
  (bind (_direction _alpha) (`Timeline|Timeline` :!via `PlayFromStart`)
    (:`Update`
      (`self.K2_SetActorLocation` (`KismetMathLibrary.VLerp` (`self.K2_GetActorLocation`) _newposition _alpha) true))
    (:`Finished`
      (`KismetSystemLibrary.Delay` (`KismetMathLibrary.RandomFloatInRange` 0.1 1.0))
      (`self.Move`))))

(fn `GetNewPosition`
  (returns (NewPosition :type "Vector Structure"))
  (bind (_currentposition_x _currentposition_y _currentposition_z) (`KismetMathLibrary.BreakVector` (`self.CurrentPosition`)))
  (return (`KismetMathLibrary.MakeVector` (+ _currentposition_x (`KismetMathLibrary.RandomIntegerInRange` (`self.Min_X`) (`self.Max_X`))) _currentposition_y (+ _currentposition_z (`KismetMathLibrary.RandomIntegerInRange` (`self.Min_Z`) (`self.Max_Z`))))))

(fn `UserConstructionScript`)