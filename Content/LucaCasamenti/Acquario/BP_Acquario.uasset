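; BP_Acquario is an aquarium actor that displays the fish with a successful date.
; On BeginPlay or the SpawnSuccessDatingFishes event, it reads FishesPool from the GI_FishAndKiss game instance.
; For each successful entry it spawns a BP_AcquarioFish at the Glass component, passing that fish's meshes and fixed, symmetric X/Z bounds.
; The spawn logic does not clear previously spawned fish.
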(event `self.ReceiveBeginPlay`
  (bind _asgi_fish_and_kiss (cast `/Game/LucaCasamenti/GameplayFramework/GameInstances/GI_FishAndKiss` (`GameplayStatics.GetGameInstance`) :!label _label))
  (for _array_element (`/Game/LucaCasamenti/GameplayFramework/GameInstances/GI_FishAndKiss.FishesPool` _asgi_fish_and_kiss)
    (if (`.successDate?_36_7311C0D2419F010DF5173AB5DF0F1B90` (break `/Game/LucaCasamenti/Fish_Finder/Structures/S_Fish` _array_element))
      (`|SpawnActorFromClass` "/Game/LucaCasamenti/Acquario/BP_AcquarioFish.BP_AcquarioFish_C" (`KismetMathLibrary.MakeTransform` (`SceneComponent.K2_GetComponentLocation` (`self.Glass`))) "Undefined" "MultiplyWithRoot" null (`.Mesh_39_9E14B6344C5D927C501C85A6AB08614F` (break `/Game/LucaCasamenti/Fish_Finder/Structures/S_Fish` _array_element)) (`.SkeletalMesh_42_5983B335410FE1EF6574AB8E7E143574` (break `/Game/LucaCasamenti/Fish_Finder/Structures/S_Fish` _array_element)) (* 90 -1) 90 (* 70 -1) 70 null))))

(event `SpawnSuccessDatingFishes`
  (goto _label))

(fn `UserConstructionScript`)