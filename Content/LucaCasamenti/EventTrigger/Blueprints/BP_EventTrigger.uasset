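; BP_EventTrigger exposes gameplay events for the Fish and Kiss game: starting fishing, opening the finder and advancing to the next fish.
; On BeginPlay it caches the GM_FishAndKiss game mode, printing an error if the cast fails.
; OpenFinder creates a new FinderDevice widget on each call and adds it to the viewport, while NextFish forwards to the game mode.
; StartFishing only prints a debug message.
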(event `self.ReceiveBeginPlay`
  ;[1 1 1] Take game mode
  (`KismetSystemLibrary.PrintString` "begin play")
  (bind _asgm_fish_and_kiss (cast `/Game/LucaCasamenti/GameModes/GM_FishAndKiss` (`GameplayStatics.GetGameMode`))
    (:`then`
      (set `self.GameMode` _asgm_fish_and_kiss))
    (:`CastFailed`
      (`KismetSystemLibrary.PrintString` "BP_EventTrigger, Non sono riuscito a prendere la game mode"))))

(event `StartFishing`
  ;[1 1 1] Start Fishing
  (`KismetSystemLibrary.PrintString` "StartFishing"))

(event `OpenFinder`
  ;[1 1 1] Open Finder
  (bind _returnvalue (`|CreateWidget` "/Game/LucaCasamenti/Finder/Widgets/FinderDevice.FinderDevice_C"))
  (bind _output_get (set `self.FinderDeviceWidget` _returnvalue))
  (`UserWidget.AddToViewport` _output_get 0))

(event `NextFish`
  ;[1 1 1] Next Fish
  (`/Game/LucaCasamenti/GameModes/GM_FishAndKiss.NextFish` (`self.GameMode`)))

(fn `UserConstructionScript`)