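; Game mode for Fish and Kiss, driving the game loop of picking a fish on a dating-style Finder tablet, catching it and decorating for the date.
; Externally triggered events switch input and cursor state, open the Finder, QTE fishing and collected-fish widgets, and spawn the caught fish.
; Fish data lives in GI_FishAndKiss, where choosing marks a fish caught.
; Date progress sums that fish's appreciation of apartment props; DecorateHome is marked unfinished.
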(event `self.ReceiveBeginPlay`
  ;[1 1 1] Get GI
  (bind _asgi_fish_and_kiss (cast `/Game/LucaCasamenti/GameplayFramework/GameInstances/GI_FishAndKiss` (`GameplayStatics.GetGameInstance`)))
  (set `self.GameInstance` _asgi_fish_and_kiss))

(event `OpenFinder`
  (bind _returnvalue (`GameplayStatics.GetPlayerController` 0))
  ;[1 1 1 0.172] Game lifecycle
  ;;[1 1 1] Open Finder
  (`self.DisableInput` (`GameplayStatics.GetPlayerPawn` 0) _returnvalue)
  (set `PlayerController.bShowMouseCursor` true _returnvalue)
  (set `PlayerController.bEnableClickEvents` true _returnvalue)
  (`/Game/LucaCasamenti/GameplayFramework/GameInstances/GI_FishAndKiss.NextFish` (`self.GameInstance`))
  (bind _returnvalue_2 (`|CreateWidget` "/Game/LucaCasamenti/Finder/Widgets/FinderDevice.FinderDevice_C" (`GameplayStatics.GetPlayerController` 0)))
  (bind _output_get (set `self.FinderTabletWidgetRef` _returnvalue_2))
  (`UserWidget.AddToViewport` _output_get 0))

(event `ChooseFishOnFinder`
  (bind _returnvalue (`GameplayStatics.GetPlayerController` 0))
  ;[1 1 1 0.172] Game lifecycle
  ;;[1 1 1] Date a fish
  (bind _fish (`/Game/LucaCasamenti/GameplayFramework/GameInstances/GI_FishAndKiss.GetFishInFocus` (`self.GameInstance`)))
  (`KismetArrayLibrary.Array_Set` (`/Game/LucaCasamenti/GameplayFramework/GameInstances/GI_FishAndKiss.FishesPool` (`self.GameInstance`)) (`self.FishesPoolCurrentIndex`) (make `/Game/LucaCasamenti/Fish_Finder/Structures/S_Fish` (break `/Game/LucaCasamenti/Fish_Finder/Structures/S_Fish` _fish) (`.Name_9_F79A53BE47F503FFC775239A5E38C591` (break `/Game/LucaCasamenti/Fish_Finder/Structures/S_Fish` _fish)) (`.FinderImage_27_8B8A7A7848BB5F30D10C54B56C140C00` (break `/Game/LucaCasamenti/Fish_Finder/Structures/S_Fish` _fish)) (`.Image_30_AF62B02443E55320F490E79286219F8C` (break `/Game/LucaCasamenti/Fish_Finder/Structures/S_Fish` _fish)) true (`.FurnitureAppreciation_26_7510560D42F8D3B90AAAD7B868E512C8` (break `/Game/LucaCasamenti/Fish_Finder/Structures/S_Fish` _fish))))
  (`self.EnableInput` (`GameplayStatics.GetPlayerPawn` 0) _returnvalue)
  (set `PlayerController.bShowMouseCursor` false _returnvalue)
  (set `PlayerController.bEnableClickEvents` false _returnvalue)
  (`self.StartCatching`))

(event `StartCatching`
  ;[1 1 1 0.172] Game lifecycle
  ;;[1 1 1] Catch fish
  (bind _returnvalue (`|CreateWidget` "/Game/DavideZanfardino/BP/HUD/Fish/W_QTEfishing.W_QTEfishing_C" null (500.0 500.0)))
  (`UserWidget.AddToViewport` _returnvalue 0)
  (`WidgetBlueprintLibrary.SetInputMode_UIOnlyEx` (`GameplayStatics.GetPlayerController` 0) _returnvalue))

(event `FinishCatching`
  (bind (_returnvalue_x _returnvalue_y _returnvalue_z) (`KismetMathLibrary.BreakVector` (`self.K2_GetActorLocation` (`self.FishermanRef`))))
  ;[1 1 1 0.172] Game lifecycle
  ;;[1 1 1] Finish Catching
  (`self.DisableInput` (`GameplayStatics.GetPlayerPawn` 0) (`GameplayStatics.GetPlayerController` 0))
  (bind _returnvalue (`|SpawnActorFromClass` "/Game/LucaCasamenti/Fish_Caught/Blueprints/BP_CaughtFish.BP_CaughtFish_C" (`KismetMathLibrary.MakeTransform` (`KismetMathLibrary.MakeVector` _returnvalue_x (+ _returnvalue_y 250.0) (- _returnvalue_z 200.0))) "Undefined" "MultiplyWithRoot" null null))
  (set `self.CaughtFishRef` _returnvalue)
  (`GameplayStatics.PlaySound2D` "/Game/LucaCasamenti/Fish_Caught/Swoundwaves/SW_Splash.SW_Splash" 1.0 1.0 0.2 null null)
  (`SkeletalMeshComponent.Stop` (`/Game/LucaCasamenti/Fisherman/Blueprints/BP_SittingFisherman.Rod` (`self.FishermanRef`))))

(event `CaughtScreen`
  ;[1 1 1 0.172] Game lifecycle
  ;;[1 1 1] Trigger caught screen
  (`KismetSystemLibrary.PrintString` "caught screen")
  (`self.K2_DestroyActor` (`self.FishermanRef`))
  (`self.K2_DestroyActor` (`self.CaughtFishRef`))
  (bind _returnvalue (`|CreateWidget` "/Game/DavideZanfardino/BP/HUD/Fish/W_FishCollected.W_FishCollected_C" null (500.0 725.0)))
  (`UserWidget.AddToViewport` _returnvalue 0))

(event `DecorateHome`
  (bind _returnvalue (`GameplayStatics.GetPlayerController` 0))
  ;[1 1 1 0.172] Game lifecycle
  ;;[1 1 1] Start decorate home
  (`KismetSystemLibrary.PrintString` "da fare")
  (`self.DisableInput` (`GameplayStatics.GetPlayerPawn` 0) _returnvalue)
  (set `PlayerController.bShowMouseCursor` true _returnvalue)
  (set `PlayerController.bEnableClickEvents` true _returnvalue)
  (set `PlayerController.bEnableMouseOverEvents` true _returnvalue))

(event `SetDateProgress`
  (`self.GetPropsInApartment`)
  (for _array_element (`self.InteractableProps`)
    (bind _fish (`/Game/LucaCasamenti/GameplayFramework/GameInstances/GI_FishAndKiss.GetFishInFocus` (`self.GameInstance`)))
    (bind (_value _returnvalue) (`BlueprintMapLibrary.Map_Find` (`.FurnitureAppreciation_26_7510560D42F8D3B90AAAD7B868E512C8` (break `/Game/LucaCasamenti/Fish_Finder/Structures/S_Fish` _fish)) (`/Game/LucaCasamenti/DecorateRoom/Blueprints/BP_InteractableProp.ActualPropType` _array_element)))
    (if _returnvalue
      (set `self.DateProgress` (+ (`self.DateProgress`) _value)))))

(fn `UserConstructionScript`)