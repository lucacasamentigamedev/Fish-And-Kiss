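; BP_AmbientSoundHandler plays 2D background music and switches tracks when the game mode requests it.
; On BeginPlay it spawns and plays the title song if no audio component exists, then binds ChangeMusic to GM_FishAndKiss through BindEventToChangeMusic.
; ChangeMusic crossfades over one second, fading out the current component and fading in a new one spawned from the game mode's NewSoundToPlay, which becomes the current component.
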(event `self.ReceiveBeginPlay`
  (`/Engine/EditorBlueprintResources/StandardMacros.IsValid` (`self.AudioComponent`)
    (:`Is Valid`
      _)
    (:`Is Not Valid`
      (bind _returnvalue (`GameplayStatics.SpawnSound2D` "/Game/DavideZanfardino/Audio/FIDH_AND_KISS_SOUND_4/MUSIC/FUNNY_TITLE_SONG.FUNNY_TITLE_SONG" 1.0 1.0 0.0 null))
      (bind _output_get (set `self.AudioComponent` _returnvalue))))
  (`AudioComponent.Play` _output_get 0.0)
  (bind _asgm_fish_and_kiss (cast `/Game/LucaCasamenti/GameplayFramework/GameModes/GM_FishAndKiss` (`GameplayStatics.GetGameMode`)))
  (add `/Game/LucaCasamenti/GameplayFramework/GameModes/GM_FishAndKiss.ChangeMusic` _asgm_fish_and_kiss (delegate `ChangeMusic`)))

(event `ChangeMusic`
  (bind _asgm_fish_and_kiss (cast `/Game/LucaCasamenti/GameplayFramework/GameModes/GM_FishAndKiss` (`GameplayStatics.GetGameMode`)))
  (`AudioComponent.FadeOut` (`self.AudioComponent`) 1.0 0.0 "Linear")
  (bind _returnvalue (`GameplayStatics.SpawnSound2D` (`/Game/LucaCasamenti/GameplayFramework/GameModes/GM_FishAndKiss.NewSoundToPlay` _asgm_fish_and_kiss) 1.0 1.0 0.0 null))
  (bind _output_get (set `self.AudioComponent` _returnvalue))
  (`AudioComponent.FadeIn` _output_get 1.0 1.0 0.0 "Linear"))

(fn `UserConstructionScript`)