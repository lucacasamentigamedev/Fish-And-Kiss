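; Player controller for FishAndKiss that handles pause and mouse click input.
; P or Escape opens a new pause menu widget once the game mode reports the game has started.
; Left mouse press and release both trigger the game mode's cursor widget click event.
; On press, a cursor trace hitting an actor without the IntProp tag broadcasts ClearHUD.
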(event `Key|P`
  (params (Key :type "Key Structure"))
  (:`Pressed`
    (bind _asgm_fish_and_kiss (cast `/Game/LucaCasamenti/GameplayFramework/GameModes/GM_FishAndKiss` (`GameplayStatics.GetGameMode`) :!label _label))
    (if (`/Game/LucaCasamenti/GameplayFramework/GameModes/GM_FishAndKiss.IsGameStarted?` _asgm_fish_and_kiss)
      (bind _returnvalue (`|CreateWidget` "/Game/DavideZanfardino/BP/HUD/PauseMenu/WI_PauseMenu.WI_PauseMenu_C"))
      (`UserWidget.AddToViewport` _returnvalue 0))))

(event `Key|Escape`
  (params (Key :type "Key Structure"))
  (:`Pressed`
    (goto _label)))

(event `Key|LeftMouseButton` :consume false
  (params (Key :type "Key Structure"))
  (bind (_hitresult _returnvalue) (`self.GetHitResultUnderCursorByChannel` "TraceTypeQuery1"))
  (:`Pressed`
    (bind _asgm_fish_and_kiss (cast `/Game/LucaCasamenti/GameplayFramework/GameModes/GM_FishAndKiss` (`GameplayStatics.GetGameMode`)))
    (`/Game/DavideZanfardino/BP/HUD/W_Cursor.ClickEvent` (`/Game/LucaCasamenti/GameplayFramework/GameModes/GM_FishAndKiss.CursorWidget` _asgm_fish_and_kiss))
    (if _returnvalue
      (if (not (`self.ActorHasTag` (`.HitActor` (`GameplayStatics.BreakHitResult` _hitresult)) "IntProp"))
        (`self.ClearHUD`))))
  (:`Released`
    (bind _asgm_fish_and_kiss_2 (cast `/Game/LucaCasamenti/GameplayFramework/GameModes/GM_FishAndKiss` (`GameplayStatics.GetGameMode`)))
    (`/Game/DavideZanfardino/BP/HUD/W_Cursor.ClickEvent` (`/Game/LucaCasamenti/GameplayFramework/GameModes/GM_FishAndKiss.CursorWidget` _asgm_fish_and_kiss_2))))

(fn `UserConstructionScript`)